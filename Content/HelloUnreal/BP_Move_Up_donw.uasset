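; BP_Move_Up_donw is a Blueprint that bobs its Cube component up and down continuously.
; Each Tick it shifts the cube along relative Z by a fixed step, using the Right boolean as the direction flag (true means up).
; The flag flips on reaching END or dropping below zero.
; The step ignores delta time, so speed depends on frame rate, and movement does not sweep for collision.
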(event `self.ReceiveTick`
  (params (DeltaSeconds :type "Float (single-precision)"))
  (bind _cube (`self.Cube`))
  (bind (_relativelocation_x _relativelocation_y _relativelocation_z) (`KismetMathLibrary.BreakVector` (`SceneComponent.RelativeLocation` _cube)))
  (bind (_relativelocation_x_2 _relativelocation_y_2 _relativelocation_z_2) (`KismetMathLibrary.BreakVector` (`SceneComponent.RelativeLocation` _cube)))
  (if (`self.Right`)
    (`SceneComponent.K2_AddRelativeLocation` _cube (0.0 0.0 5.0) false false)
    (if (>= _relativelocation_z_2 (`self.END`))
      (set `self.Right` false))
    (else
      (`SceneComponent.K2_AddRelativeLocation` (`self.Cube`) (0.0 0.0 -5.0) false false)
      (if (< _relativelocation_z 0.0)
        (set `self.Right` true)))))

(fn `UserConstructionScript`)